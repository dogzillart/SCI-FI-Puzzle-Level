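; Vent elevator interactable whose Elevator component extends and retracts vertically with its power state.
; Power update events from the parent feed UpdatePositions, which lerps between MinHeight and Height, and the finish event snaps to the Active state.
; Z scale and a half-height offset change together, so a centered 100-unit mesh grows from a fixed base.
; SetupMaterialOwners applies MainPowerMaterial to the Elevator.
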(event EventBeginPlay
  (|CallParentFunction))

(event Collision|EventActorBeginOverlap
  (params (OtherActor :type Actor%20Object%20Reference))
  (|CallParentFunction OtherActor) ; This node is disabled and will not be called.\nDrag off pins to build functionality.
)

(event EventTick
  (params (DeltaSeconds :type Float%20%28single-precision%29))
  (|CallParentFunction DeltaSeconds) ; This node is disabled and will not be called.\nDrag off pins to build functionality.
)

(event EventSetupMaterialOwners
  (Rendering|Material|SetMaterial (Variables|Default|GetElevator) 0 (Variables|Default|GetMain%20Power%20Material)))

(event EventOnUpdatePowerUpdate
  (params (Current%20Amount :type Float%20%28single-precision%29))
  (CallFunction|UpdatePositions Current%20Amount))

(event EventOnUpdatePowerFinished
  (params (Forced :type Boolean))
  (CallFunction|UpdatePositions (Math|Conversions|ToFloat(Boolean) (Variables|Default|GetActive))))

(fn ConstructionScript
  (|CallParentFunction))

(fn UpdatePositions
  (params (Amount :type Float%20%28single-precision%29))
  (bind _height (Variables|Default|GetHeight))
  (bind _minheight (Variables|Default|GetMinHeight))
  (bind _returnvalue (Math|Float|Lerp _minheight _height Amount))
  (Transformation|SetRelativeLocation (Variables|Default|GetElevator) (Math|Vector|MakeVector 0.0 0.0 (/ _returnvalue 2.0)) false false)
  (Transformation|SetRelativeScale3D (Variables|Default|GetElevator) (Math|Vector|MakeVector 1.0 1.0 (/ _returnvalue 1e+02))))