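; Prototype vent fan whose spinning part and box collision respond to an activation flag read from an Active reference.
; BeginPlay binds the rotating movement component to the fan part.
; While DidActivate is true, Tick plays a timeline that drives rotation speed.
; Its update path also runs a five-second Delay, then disables box collision, toggles the movement component and stops the timeline, which Tick can restart.
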(event EventBeginPlay
  (Components|Movement|SetUpdatedComponent (Variables|Default|GetFan%20Rotation) (Variables|Default|GetSpinning%20Fan%20Part)))

(event EventTick
  (params (DeltaSeconds :type Float%20%28single-precision%29))
  (if (Variables|/Game/FPPTemplate/Blueprints/LogicGates/BP_FPPT_DoOnceGate.BP_FPPT_DoOnceGate_C|GetDidActivate (Variables|Default|GetActive))
    (bind _rotationspped (Timeline|RotateFan Play)
      (:Update
        (Variables|/Script/Engine.RotatingMovementComponent|SetRotationRate (Variables|Default|GetFan%20Rotation) (Math|Rotator|MakeRotator _rotationspped 0.0 0.0))
        (Utilities|FlowControl|Delay 5.0)
        (Collision|SetCollisionEnabled (Variables|Default|GetBox) "NoCollision")
        (Components|Activation|ToggleActive (Variables|Default|GetFan%20Rotation))
        (Timeline|RotateFan Stop)))))

(fn ConstructionScript)

(fn NewFunction0)